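; Game instance that holds the player profile, vehicle and color catalogs, level progress and money for a vehicle game.
; On Init it builds UObjects from data tables, then loads or creates the save and applies saved volumes through a sound mix.
; Level rewards shrink by HP-range penalties from a rewards table.
; Purchases, level completion and active-vehicle changes update the profile and trigger an async save.
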(event Custom|Event%20Save%20Profile
  (bind _savegameinst (Variables|Default|GetSaveGameInst))
  ;[1 1 1] Event save current player profile
  (Default|SaveProfile _savegameinst (Variables|Default|GetPlayerProfile))
  (|AsyncSaveGametoSlot _savegameinst (Variables|Default|GetPlayerProfileSave)))

(event Custom|Event%20Finished%20Current%20Level
  (Variables|/Game/GameBP/Blueprints/Gameplay/Objects/BP_Profile_Obj.BP_Profile_Obj_C|SetCurLevel (Variables|Default|GetPlayerProfile) (Variables|Levels|GetNextLevel))
  (CallFunction|EventSaveProfile))

(event Custom|Event%20Buy%20Vehicle
  (params (NewVehicle :type BP%20Vehicle%20Obj%20Object%20Reference%20%28by%20ref%29) (NewColor :type BP%20Vehicle%20Color%20Obj%20Object%20Reference%20%28by%20ref%29))
  (bind _playerprofile (Variables|Default|GetPlayerProfile))
  ;[1 1 1] Bought new vehicle with in-game money
  (Default|DecreaseMoney _playerprofile (Variables|/Game/GameBP/Blueprints/Gameplay/Objects/BP_Vehicle_Obj.BP_Vehicle_Obj_C|GetPrice NewVehicle))
  (Default|AddVehiclewithColor _playerprofile (Variables|/Game/GameBP/Blueprints/Gameplay/Objects/BP_Vehicle_Obj.BP_Vehicle_Obj_C|GetId NewVehicle) (Variables|/Game/GameBP/Blueprints/Gameplay/Objects/BP_VehicleColor_Obj.BP_VehicleColor_Obj_C|GetId NewColor))
  (CallFunction|EventSaveProfile))

(event Custom|Event%20Buy%20Color%20For%20Vehicle
  (params (New%20Color :type BP%20Vehicle%20Color%20Obj%20Object%20Reference) (Vehicle :type BP%20Vehicle%20Obj%20Object%20Reference))
  (bind _playerprofile (Variables|Default|GetPlayerProfile))
  ;[1 1 1] Bought new vehicle with in-game money
  (Default|DecreaseMoney _playerprofile (Variables|/Game/GameBP/Blueprints/Gameplay/Objects/BP_VehicleColor_Obj.BP_VehicleColor_Obj_C|GetPrice New%20Color))
  (Default|AddColorforVehicle _playerprofile (Variables|/Game/GameBP/Blueprints/Gameplay/Objects/BP_VehicleColor_Obj.BP_VehicleColor_Obj_C|GetId New%20Color) (Variables|/Game/GameBP/Blueprints/Gameplay/Objects/BP_Vehicle_Obj.BP_Vehicle_Obj_C|GetId Vehicle))
  (CallFunction|EventSaveProfile))

(event EventInit
  ;[1 1 1] Init game - preload data -- save game
  (Economy|LoadRewardsData)
  (Data|LoadAllData)
  (Development|ExecuteConsoleCommand "r.ShadowQuality 0" 0))

(fn GetNextLevel
  (bind _output_get (Variables|Levels|SetNextLevel (+ (Levels|GetCurrentLevel) 1)))
  (return _output_get))

(fn GetCurrentMoney
  (return (Variables|/Game/GameBP/Blueprints/Gameplay/Objects/BP_Profile_Obj.BP_Profile_Obj_C|GetMoney (Variables|Default|GetPlayerProfile))))

(fn LoadRewardsData
  (bind _outrownames (DataTable|GetDataTableRowNames "/Game/GameData/Data/DT_PlayerRewards.DT_PlayerRewards"))
  (for _array_element _outrownames
    (bind _returnvalue (Utilities|GetDataTableRow "/Game/GameData/Data/DT_PlayerRewards.DT_PlayerRewards" _array_element)
      (:then
        (Utilities|Array|Add (Variables|Default|GetPlayerRewardsData) _returnvalue)))))

(fn UpdateMoney
  (params (PlayerHP :type Float%20%28single-precision%29) (Bonus :type Integer))
  (bind _rewardperlevel (Variables|Default|GetRewardPerLevel))
  (for _array_element (Variables|Default|GetPlayerRewardsData)
    (if (Math|Float|InRange(Float) PlayerHP (.lowerplayerhp _array_element) (.upperplayerhp _array_element))
      (Default|AddMoney (Variables|Default|GetPlayerProfile) (+ (Math|Float|Ceil (- _rewardperlevel (* (.moneypenalty _array_element) _rewardperlevel))) Bonus))
      (return (+ (Math|Float|Ceil (- _rewardperlevel (* (.moneypenalty _array_element) _rewardperlevel))) Bonus) (Math|Float|Ceil (* (.moneypenalty _array_element) _rewardperlevel))))))

(fn LoadSaveGame
  (bind _returnvalue (SaveGame|DoesSaveGameExist (Variables|Default|GetPlayerProfileSave)))
  (if _returnvalue
    (bind _returnvalue_2 (SaveGame|LoadGamefromSlot (Variables|Default|GetPlayerProfileSave)))
    (bind _asbp_main_save_game (Utilities|Casting|CastToBP_MainSaveGame _returnvalue_2))
    (LocalVariables|SetMainSaveGameInst _asbp_main_save_game)
    (else
      (bind _returnvalue_3 (SaveGame|CreateSaveGameObject "/Game/GameBP/Blueprints/BP_MainSaveGame.BP_MainSaveGame_C"))
      (LocalVariables|SetMainSaveGameInst _returnvalue_3)))
  (return _returnvalue (LocalVariables|GetMainSaveGameInst)))

(fn GetCurrentLevel
  (return (Variables|/Game/GameBP/Blueprints/Gameplay/Objects/BP_Profile_Obj.BP_Profile_Obj_C|GetCurLevel (Variables|Default|GetPlayerProfile))))

(fn ToggleGameplayState
  (params (IsInGameplay :type Boolean))
  (bind _output_get (Variables|Levels|SetIsInGameplay IsInGameplay))
  (return _output_get))

(fn GetGameplayState
  (return (Variables|Levels|GetIsInGameplay)))

(fn GetColorbyId
  (params (ColorId :type Integer))
  (bind _vehiclecolors (Variables|Data|GetVehicleColors))
  (bind (_value _returnvalue) (Utilities|Map|Find _vehiclecolors ColorId))
  (if _returnvalue
    (return _value)))

(fn AddNewVehicle
  (params (Vehicle :type BP%20Vehicle%20Obj%20Object%20Reference%20%28by%20ref%29) (VehicleColor :type BP%20Vehicle%20Color%20Obj%20Object%20Reference%20%28by%20ref%29))
  (Default|AddVehiclewithColor (Variables|Default|GetPlayerProfile) (Variables|/Game/GameBP/Blueprints/Gameplay/Objects/BP_Vehicle_Obj.BP_Vehicle_Obj_C|GetId Vehicle) (Variables|/Game/GameBP/Blueprints/Gameplay/Objects/BP_VehicleColor_Obj.BP_VehicleColor_Obj_C|GetId VehicleColor)))

(fn InitProfile
  (params (ProfileData :type ST%20Player%20Profile%20Structure) (OwnedVehicles :type Map%20of%20Integers%20to%20Structs))
  (bind _returnvalue (Game|ConstructObjectfromClass "/Game/GameBP/Blueprints/Gameplay/Objects/BP_Profile_Obj.BP_Profile_Obj_C" self))
  (bind _newprofile (Default|InitwithData _returnvalue ProfileData OwnedVehicles))
  (bind _output_get (Variables|Default|SetPlayerProfile _newprofile))
  (CallFunction|SetVolume "NewEnumerator0" (.mastervolume (Variables|/Game/GameBP/Blueprints/Gameplay/Objects/BP_Profile_Obj.BP_Profile_Obj_C|GetOptions _output_get)))
  (CallFunction|SetVolume "NewEnumerator1" (.musicvolume (Variables|/Game/GameBP/Blueprints/Gameplay/Objects/BP_Profile_Obj.BP_Profile_Obj_C|GetOptions _output_get)))
  (CallFunction|SetVolume "NewEnumerator2" (.sfxvolume (Variables|/Game/GameBP/Blueprints/Gameplay/Objects/BP_Profile_Obj.BP_Profile_Obj_C|GetOptions _output_get))))

(fn InitColors
  (bind _outrownames (DataTable|GetDataTableRowNames "/Game/GameData/Data/DT_Colors.DT_Colors"))
  (for _array_element _outrownames
    (bind _returnvalue (Utilities|GetDataTableRow "/Game/GameData/Data/DT_Colors.DT_Colors" _array_element)
      (:then
        (bind _returnvalue_2 (Game|ConstructObjectfromClass "/Game/GameBP/Blueprints/Gameplay/Objects/BP_VehicleColor_Obj.BP_VehicleColor_Obj_C" self))
        (bind _newcolor (Default|InitwithData _returnvalue_2 _returnvalue))
        (Utilities|Map|Add (Variables|Data|GetVehicleColors) (Variables|/Game/GameBP/Blueprints/Gameplay/Objects/BP_VehicleColor_Obj.BP_VehicleColor_Obj_C|GetId _newcolor) _newcolor)))))

(fn InitVehicles
  (bind _outrownames (DataTable|GetDataTableRowNames "/Game/GameData/Data/DT_Vehicles.DT_Vehicles"))
  (for _array_element _outrownames
    (bind _returnvalue (Utilities|GetDataTableRow "/Game/GameData/Data/DT_Vehicles.DT_Vehicles" _array_element)
      (:then
        (bind _returnvalue_2 (Game|ConstructObjectfromClass "/Game/GameBP/Blueprints/Gameplay/Objects/BP_Vehicle_Obj.BP_Vehicle_Obj_C" self))
        (bind _newvehicle (Default|InitwithData _returnvalue_2 _returnvalue))
        (Utilities|Map|Add (Variables|Data|GetVehicles) (Variables|/Game/GameBP/Blueprints/Gameplay/Objects/BP_Vehicle_Obj.BP_Vehicle_Obj_C|GetId _newvehicle) _newvehicle)))))

(fn LoadAllData
  (Data|InitColors)
  (bind (_exists _savegame) (Gameplay|LoadSaveGame))
  (Variables|Default|SetSaveGameInst _savegame)
  (if _exists
    (Data|InitVehicles)
    (Data|InitProfile (Variables|/Game/GameBP/Blueprints/BP_MainSaveGame.BP_MainSaveGame_C|GetSavedPlayerProfile (Variables|Default|GetSaveGameInst)) (Variables|/Game/GameBP/Blueprints/BP_MainSaveGame.BP_MainSaveGame_C|GetOwnedVehicles (Variables|Default|GetSaveGameInst)))
    (else
      (Data|InitVehicles)
      (Data|InitProfile :OwnedVehicles (Utilities|Map|MakeMap 1 (Utilities|Struct|MakeST_IntLIst (Utilities|Array|MakeArray 0)))))))

(fn GetActiveVehicle
  (bind _playerprofile (Variables|Default|GetPlayerProfile))
  (return (Vehicle|GetVehiclebyId (Variables|/Game/GameBP/Blueprints/Gameplay/Objects/BP_Profile_Obj.BP_Profile_Obj_C|GetActiveVehicleId _playerprofile)) (Color|GetColorbyId (Variables|/Game/GameBP/Blueprints/Gameplay/Objects/BP_Profile_Obj.BP_Profile_Obj_C|GetActiveColorId _playerprofile))))

(fn GetVehiclebyId
  (params (Id :type Integer))
  (bind _vehicles (Variables|Data|GetVehicles))
  (bind (_value _returnvalue) (Utilities|Map|Find _vehicles Id))
  (if _returnvalue
    (return _value)))

(fn SetActiveVehicle
  (params (PickedVehicle :type BP%20Vehicle%20Obj%20Object%20Reference%20%28by%20ref%29))
  (bind _playerprofile (Variables|Default|GetPlayerProfile))
  (Variables|/Game/GameBP/Blueprints/Gameplay/Objects/BP_Profile_Obj.BP_Profile_Obj_C|SetActiveVehicleId _playerprofile (Variables|/Game/GameBP/Blueprints/Gameplay/Objects/BP_Vehicle_Obj.BP_Vehicle_Obj_C|GetId PickedVehicle))
  (Variables|/Game/GameBP/Blueprints/Gameplay/Objects/BP_Profile_Obj.BP_Profile_Obj_C|SetActiveColorId _playerprofile (Variables|/Game/GameBP/Blueprints/Gameplay/Objects/BP_Vehicle_Obj.BP_Vehicle_Obj_C|GetActiveColorId PickedVehicle))
  (CallFunction|EventSaveProfile))

(fn IsVehicleOwned
  (params (Id :type Integer))
  (return (Default|IsVehicleOwned (Variables|Default|GetPlayerProfile) Id)))

(fn IsVehicleColorOwned
  (params (VehicleId :type Integer) (ColorId :type Integer))
  (return (Default|IsVehicleColorOwned (Variables|Default|GetPlayerProfile) VehicleId ColorId)))

(fn SetVolume
  (params (AudioType :type ENUM_AudioTypes%20Enum :default "NewEnumerator0") (Value :type Float%20%28single-precision%29))
  (switch Utilities|FlowControl|Switch|SwitchonENUM_AudioTypes AudioType
    (:NewEnumerator0
      (LocalVariables|SetSoundClass "/Game/GameBP/Blueprints/Gameplay/Effects/SFX/SC_Master.SC_Master"))
    (:NewEnumerator1
      (LocalVariables|SetSoundClass "/Game/GameBP/Blueprints/Gameplay/Effects/SFX/SC_BackgroundMusic.SC_BackgroundMusic"))
    (:NewEnumerator2
      (LocalVariables|SetSoundClass "/Game/GameBP/Blueprints/Gameplay/Effects/SFX/SC_Sfx.SC_Sfx")))
  (Audio|SetSoundMixClassOverride "/Game/GameBP/Blueprints/Gameplay/Effects/SFX/SM_MasterMix.SM_MasterMix" (LocalVariables|GetSoundClass) Value 1.0 1.0 true))