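; Base vehicle Blueprint that exposes throttle, stop and steering events and prepares speed (km/h) and gear (R/N/number) strings for a HUD each tick.
; Throttle applies half input and forces the body's X velocity to MaxSpeed, while Stop zeroes throttle and velocity.
; Steering bypasses wheel input, pushing the body with a signed velocity-change impulse on Y and half that on X.
; Handbrake calls exist but are unwired.
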(event Custom|Event%20Update%20Steering%20Direction
  (params (Direction :type Directions%20Enum :default "NewEnumerator0"))
  ;[1 1 1] Steering Input + Direction
  (Input|UpdateSteering Direction))

(event Custom|Event%20Update%20Acceleration
  (params (Amount :type Float%20%28single-precision%29))
  (bind _vehiclemovement (Variables|Default|GetVehicleMovement))
  ;[1 1 1] Throttle input
  (Class|WheeledVehicleMovementComponent|SetThrottleInput _vehiclemovement 0.5)
  (Physics|SetPhysicsLinearVelocity (Variables|/Script/Engine.MovementComponent|GetUpdatedPrimitive _vehiclemovement) (Math|Vector|MakeVector (Variables|Config|GetMaxSpeed) 0.0 0.0) false "None"))

(event Custom|Event%20Stop
  ;[1 1 1] Auto brake when idle is seti via VehicleMovement comp settings
  (Class|WheeledVehicleMovementComponent|SetThrottleInput (Variables|Default|GetVehicleMovement) 0.0)
  (Physics|SetPhysicsLinearVelocity (Variables|/Script/Engine.MovementComponent|GetUpdatedPrimitive (Variables|Default|GetVehicleMovement)) "0, 0, 0" false "None"))

(event EventTick
  (params (DeltaSeconds :type Float%20%28single-precision%29))
  ;[1 0.4422 0.03086] On tick - KM/H update
  (Variables|Game|SetInReverseGear (< (Class|WheeledVehicleMovementComponent|GetCurrentGear (Variables|Default|GetVehicleMovement)) 0))
  (HUD|UpdateHUDStrings))

(event Input|ActionEvents|InputActionHandbrake
  (params (Key :type Key%20Structure :default "None"))
  ;[0.6771 0.006217 0] Handbrake input
)

(fn ConstructionScript)

(fn ResetSteering
  (if (Variables|Input|GetIsSteering)
    (Class|WheeledVehicleMovementComponent|SetSteeringInput (Variables|Default|GetVehicleMovement) 0.0)))

(fn UpdateSteering
  (params (Direction :type Directions%20Enum :default "NewEnumerator0"))
  (switch Utilities|FlowControl|Switch|SwitchonDirections Direction
    (:NewEnumerator0
      (LocalVariables|SetDirectionMultiplier -1.0))
    (:NewEnumerator1
      (LocalVariables|SetDirectionMultiplier 1.0)))
  (bind _output_get (LocalVariables|SetFinalImpulse (* (Variables|Input|GetSteerVelocityMultiplier) (LocalVariables|GetDirectionMultiplier))))
  (Physics|AddImpulse (Variables|/Script/Engine.MovementComponent|GetUpdatedPrimitive (Variables|Default|GetVehicleMovement)) (Math|Vector|MakeVector (/ (* (Variables|Input|GetSteerVelocityMultiplier) (LocalVariables|GetDirectionMultiplier)) 2.0) _output_get 0.0) "None" true)
  (return))

(fn UpdateHUDStrings
  ;[1 1 1] Setup String for Speed
  (Variables|HUD|SetSpeed%20Display%20String (Utilities|String|Append (Utilities|String|ToString(Integer) (CallFunction|GetReadableSpeed)) " km/h"))
  ;[1 1 1] Setup string for Gear
  (LocalVariables|SetCurrentGear (Class|WheeledVehicleMovementComponent|GetCurrentGear (Variables|Default|GetVehicleMovement)))
  (if (Variables|Game|GetInReverseGear) ; If zero display N else display R
    (Variables|HUD|SetGear%20Display%20String "R")
    (elif (> (LocalVariables|GetCurrentGear) 0) ; If the gear is above zero use that
      (Variables|HUD|SetGear%20Display%20String (Utilities|String|ToString(Integer) (LocalVariables|GetCurrentGear)))
      (else
        (Variables|HUD|SetGear%20Display%20String "N")))))

(fn GetReadableSpeed
  (return (Math|Float|Floor (Math|Float|Absolute(Float) (* (Class|WheeledVehicleMovementComponent|GetForwardSpeed (Variables|Default|GetVehicleMovement)) 0.036)))))