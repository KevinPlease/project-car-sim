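; BP_Animal is an animal character that goes limp when a vehicle reaches it.
; The first proximity overlap by a BP_BaseVehicle turns on mesh physics simulation and destroys the capsule, though DoOnce is consumed by any first overlapping actor.
; Construction copies Mass into CharacterMovement.
; InitPhysics, not called here, sets up physical animation with torso settings on simulated bodies below the root bone.
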(event OnComponentBeginOverlap(ProximityCollision)
  (params (OverlappedComponent :type Primitive%20Component%20Object%20Reference) (OtherActor :type Actor%20Object%20Reference) (OtherComp :type Primitive%20Component%20Object%20Reference) (OtherBodyIndex :type Integer) (bFromSweep :type Boolean) (SweepResult :type Hit%20Result%20Structure%20%28by%20ref%29))
  (Utilities|FlowControl|DoOnce false
    (:Completed
      (Utilities|Casting|CastToBP_BaseVehicle OtherActor)
      (Physics|SetSimulatePhysics (Variables|Character|GetMesh) true)
      (Components|DestroyComponent (Variables|Collision|GetCapsuleComponent)))))

(fn ConstructionScript
  (Variables|/Script/Engine.CharacterMovementComponent|SetMass (Variables|Character|GetCharacterMovement) (Variables|Default|GetMass)))

(fn InitPhysics
  (bind _rootbonename (Variables|Default|GetRootBoneName))
  (Class|PhysicalAnimationComponent|SetSkeletalMeshComponent (Variables|Default|GetPhysicalAnimation) (Variables|Character|GetMesh))
  ;[1 1 1] Config Torso Physics
  (Class|PhysicalAnimationComponent|ApplyPhysicalAnimationSettingsBelow (Variables|Default|GetPhysicalAnimation) _rootbonename (Variables|Default|GetTorsoPhysicsSettings) false)
  (Class|SkeletalMeshComponent|SetAllBodiesBelowSimulatePhysics (Variables|Character|GetMesh) _rootbonename true false))