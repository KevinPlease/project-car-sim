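; Pedestrian character whose skeletal mesh blends animation with physics simulation through a PhysicalAnimation component.
; On BeginPlay it caches its AnimBP_Pedestrian instance, then InitPhysics applies separate torso and leg settings and simulates the bodies below those root bones, excluding the roots.
; The construction script sets movement mass from Weight, scales the capsule by Height and shows mass as debug text.
; The Hit handler checks for I_Player but takes no action yet.
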(event EventBeginPlay
  ;[1 1 1] Begin Play
  (bind _asanim_bp_pedestrian (Utilities|Casting|CastToAnimBP_Pedestrian (Components|SkeletalMesh|GetAnimInstance (Variables|Character|GetMesh))))
  (Variables|Default|SetAnimInstance _asanim_bp_pedestrian)
  (CallFunction|InitPhysics))

(event Collision|EventHit
  (params (MyComp :type Primitive%20Component%20Object%20Reference) (Other :type Actor%20Object%20Reference) (OtherComp :type Primitive%20Component%20Object%20Reference) (bSelfMoved :type Boolean) (HitLocation :type Vector :default "0, 0, 0") (HitNormal :type Vector :default "0, 0, 0") (NormalImpulse :type Vector :default "0, 0, 0") (Hit :type Hit%20Result%20Structure%20%28by%20ref%29))
  (if (Utilities|DoesObjectImplementInterface Other "/Game/GameBP/Blueprints/Gameplay/Interfaces/I_Player.I_Player_C")
    _))

(fn ConstructionScript
  (bind _height (Variables|Stats|GetHeight))
  (Variables|/Script/Engine.CharacterMovementComponent|SetMass (Variables|Character|GetCharacterMovement) (Variables|Stats|GetWeight))
  (Transformation|SetWorldScale3D (Variables|Collision|GetCapsuleComponent) (Math|Vector|MakeVector _height _height _height))
  ;[1 0.535 0.1096] TODO: DEBUGGING
  (Rendering|Components|TextRender|SetText (Variables|Default|GetTextRender) (Utilities|Text|ToText(Float) (Variables|/Script/Engine.CharacterMovementComponent|GetMass (Variables|Character|GetCharacterMovement)) "HalfToEven" false true 1 324 0 0)))

(fn InitPhysics
  (bind _legphysicssettings (Variables|Physics|GetLegPhysicsSettings))
  (bind _legrootbone_l (Variables|Physics|GetLegRootBone_L))
  (bind _legrootbone_r (Variables|Physics|GetLegRootBone_R))
  (bind _torsorootbone (Variables|Physics|GetTorsoRootBone))
  (bind _physicalanimation (Variables|Default|GetPhysicalAnimation))
  (bind _mesh (Variables|Character|GetMesh))
  (Class|PhysicalAnimationComponent|SetSkeletalMeshComponent (Variables|Default|GetPhysicalAnimation) (Variables|Character|GetMesh))
  (Utilities|FlowControl|Sequence
    (:then_0
      ;[1 1 1] Config Torso Physics
      (Class|PhysicalAnimationComponent|ApplyPhysicalAnimationSettingsBelow _physicalanimation _torsorootbone (Variables|Physics|GetTorsoPhysicsSettings) false)
      (Class|SkeletalMeshComponent|SetAllBodiesBelowSimulatePhysics _mesh _torsorootbone true false))
    (:then_1
      ;[1 1 1] Config Left Leg Physics
      (Class|PhysicalAnimationComponent|ApplyPhysicalAnimationSettingsBelow _physicalanimation _legrootbone_l _legphysicssettings false)
      (Class|SkeletalMeshComponent|SetAllBodiesBelowSimulatePhysics _mesh _legrootbone_l true false))
    (:then_2
      ;[1 1 1] Config Right Leg Physics
      (Class|PhysicalAnimationComponent|ApplyPhysicalAnimationSettingsBelow (Variables|Default|GetPhysicalAnimation) _legrootbone_r _legphysicssettings false)
      (Class|SkeletalMeshComponent|SetAllBodiesBelowSimulatePhysics (Variables|Character|GetMesh) _legrootbone_r true false))))