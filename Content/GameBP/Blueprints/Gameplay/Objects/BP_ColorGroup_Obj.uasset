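; BP_ColorGroup_Obj is a data object that holds one color group and the vehicle colors belonging to it.
; InitWithData stores the group data, caches its type as the group identifier, sets the color list and returns itself.
; Helper functions append a color, test whether a color is in the list, and find a color by Id through a linear search that also reports a found flag.
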(fn InitwithData
  (params (ColorTypeData :type ST%20Color%20Group%20Structure) (VehicleColors :type Array%20of%20BP%20Vehicle%20Color%20Obj%20Object%20References))
  (bind _output_get (Variables|Default|SetColorGroupData ColorTypeData))
  (Variables|Default|SetColorGroup (.type _output_get))
  (Variables|Default|SetVehicleColors VehicleColors)
  (return self))

(fn AddColor
  (params (NewColor :type BP%20Vehicle%20Color%20Obj%20Object%20Reference%20%28by%20ref%29))
  (Utilities|Array|Add (Variables|Default|GetVehicleColors) NewColor))

(fn ContainsColor
  (params (Color :type BP%20Vehicle%20Color%20Obj%20Object%20Reference%20%28by%20ref%29))
  (return (Utilities|Array|ContainsItem (Variables|Default|GetVehicleColors) Color)))

(fn GetColorbyId
  (params (Id :type Integer))
  (for _array_element (Variables|Default|GetVehicleColors)
    (if (== Id (Variables|/Game/GameBP/Blueprints/Gameplay/Objects/BP_VehicleColor_Obj.BP_VehicleColor_Obj_C|GetId _array_element))
      (return _array_element (== Id (Variables|/Game/GameBP/Blueprints/Gameplay/Objects/BP_VehicleColor_Obj.BP_VehicleColor_Obj_C|GetId _array_element))))))