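; Tile-owned spawner that periodically spawns rows of animals of a given class, tuned by a Difficulty setting.
; Init supplies class, difficulty and parent tile; BeginSpawn starts a looping timer whose clamped interval is rolled once from the row-size range.
; Each tick spawns a random-sized row, registering animals with the tile.
; Spacing uses random difficulty distances converted by the tile, stepping along Y away from zero on the spawner's side.
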(event Custom|Event%20Begin%20Spawn
  (bind _difficulty (Variables|Default|GetDifficulty))
  (Utilities|Time|SetTimerbyEvent (delegate Custom|Event%20Spawn) (Math|Float|Clamp(Float) (* (- (Math|Random|RandomIntegerinRange (.minanimalsinrow _difficulty) (.maxanimalsinrow _difficulty)) 1) (Variables|Default|GetDefaultSpawnInterval)) 6.0 12.0) true))

(event Custom|Event%20Spawn
  (CallFunction|SpawnAnimals))

(event EventBeginPlay)

(fn ConstructionScript)

(fn SpawnAnimals
  (bind _difficulty (Variables|Default|GetDifficulty))
  (bind _output_get (LocalVariables|SetCurSpawnLoc (Transformation|GetActorTransform)))
  (for _index (range 0 (- (Math|Random|RandomIntegerinRange (.minanimalsinrow _difficulty) (.maxanimalsinrow _difficulty)) 1))
    (bind _returnvalue (Game|SpawnActorfromClass (Variables|Default|GetAnimalToSpawn) _output_get "AdjustIfPossibleButAlwaysSpawn" 0 0))
    (Variables|/Game/GameBP/Blueprints/Gameplay/Animals/BP_Animal.BP_Animal_C|SetParentTile _returnvalue (Variables|Default|GetParentTile))
    (Utilities|Array|Add (Variables|/Game/GameBP/Blueprints/Gameplay/Tiles/BP_MasterTile.BP_MasterTile_C|GetAiSpawned (Variables|Default|GetParentTile)) _returnvalue)
    (Math|Float|CompareFloat (.y (.location (LocalVariables|GetCurSpawnLoc))) 0.0
      (:>
        (LocalVariables|SetCurSpawnLoc (Math|Transform|MakeTransform (Math|Vector|MakeVector (.x (.location (LocalVariables|GetCurSpawnLoc))) (+ (Default|GetAiDistanceOffset (Variables|Default|GetParentTile) (Utilities|Array|Get(acopy) (.animaldistances _difficulty) (Math|Random|RandomIntegerinRange 0 (- (Utilities|Array|Length (.animaldistances _difficulty)) 1)))) (.y (.location (LocalVariables|GetCurSpawnLoc)))) (.z (.location (LocalVariables|GetCurSpawnLoc)))) (.rotation (LocalVariables|GetCurSpawnLoc)) (.scale (LocalVariables|GetCurSpawnLoc)))))
      (:<
        (LocalVariables|SetCurSpawnLoc (Math|Transform|MakeTransform (Math|Vector|MakeVector (.x (.location (LocalVariables|GetCurSpawnLoc))) (- (.y (.location (LocalVariables|GetCurSpawnLoc))) (Default|GetAiDistanceOffset (Variables|Default|GetParentTile) (Utilities|Array|Get(acopy) (.animaldistances _difficulty) (Math|Random|RandomIntegerinRange 0 (- (Utilities|Array|Length (.animaldistances _difficulty)) 1))))) (.z (.location (LocalVariables|GetCurSpawnLoc)))) (.rotation (LocalVariables|GetCurSpawnLoc)) (.scale (LocalVariables|GetCurSpawnLoc))))))))

(fn Init
  (params (AnimalToSpawn :type BP%20Animal%20Class%20Reference) (Difficulty :type ST%20Difficulty%20Structure) (ParentTile :type BP%20Master%20Tile%20Object%20Reference))
  (Variables|Default|SetAnimalToSpawn AnimalToSpawn)
  (Variables|Default|SetDifficulty Difficulty)
  (Variables|Default|SetParentTile ParentTile))