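; Runtime player profile object holding name, options, money, current level, active vehicle and color, and owned vehicles.
; It initializes from profile data plus an owned-vehicle map and packs the same state back into a profile struct and map for saving.
; Helpers adjust money without balance checks and add or query ownership through the map of vehicle IDs to unlocked color IDs.
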(fn InitwithData
  (params (ProfileData :type ST%20Player%20Profile%20Structure) (OwnedVehicles :type Map%20of%20Integers%20to%20Structs))
  (bind (_name _options _money _currentlevel _activevehicleid _activecolorid) (Utilities|Struct|BreakST_PlayerProfile ProfileData))
  (Variables|Default|SetUsername _name)
  (Variables|Default|SetOptions _options)
  (Variables|Vars|SetMoney _money)
  (Variables|Vars|SetCurLevel _currentlevel)
  (Variables|Vars|SetOwnedVehicles OwnedVehicles)
  (Variables|Default|SetActiveVehicleId _activevehicleid)
  (Variables|Default|SetActiveColorId _activecolorid)
  (return self))

(fn GetSaveData
  (return (Utilities|Struct|MakeST_PlayerProfile (Variables|Default|GetUsername) (Variables|Default|GetOptions) (Variables|Vars|GetMoney) (Variables|Vars|GetCurLevel) (Variables|Default|GetActiveVehicleId) (Variables|Default|GetActiveColorId)) (Variables|Vars|GetOwnedVehicles)))

(fn AddMoney
  (params (Amount :type Integer))
  (bind _output_get (Variables|Vars|SetMoney (+ Amount (Variables|Vars|GetMoney))))
  (return _output_get))

(fn DecreaseMoney
  (params (Amount :type Integer))
  (bind _output_get (Variables|Vars|SetMoney (- (Variables|Vars|GetMoney) Amount)))
  (return _output_get))

(fn AddColorforVehicle
  (params (ColorId :type Integer) (VehicleId :type Integer))
  (bind _ownedvehicles (Variables|Vars|GetOwnedVehicles))
  (bind _output_get (LocalVariables|SetLocNewColors (.ids (.Value (Utilities|Map|Find _ownedvehicles VehicleId)))))
  (Utilities|Array|AddUnique _output_get ColorId)
  (Utilities|Map|Add _ownedvehicles VehicleId (Utilities|Struct|MakeST_IntLIst (LocalVariables|GetLocNewColors))))

(fn AddVehiclewithColor
  (params (VehicleId :type Integer) (ColorId :type Integer))
  (Utilities|Map|Add (Variables|Vars|GetOwnedVehicles) VehicleId (Utilities|Struct|MakeST_IntLIst (Utilities|Array|MakeArray ColorId))))

(fn IsVehicleOwned
  (params (Id :type Integer))
  (return (.ReturnValue (Utilities|Map|Find (Variables|Vars|GetOwnedVehicles) Id))))

(fn IsVehicleColorOwned
  (params (VehicleId :type Integer) (ColorId :type Integer))
  (return (Utilities|Array|ContainsItem (.ids (.Value (Utilities|Map|Find (Variables|Vars|GetOwnedVehicles) VehicleId))) ColorId)))