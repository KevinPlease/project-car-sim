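; BP_MasterTile is the base floor tile for an endlessly spawned track, providing transforms for the next tile and for left/right obstacles.
; When a player (I_Player) first overlaps EndOfTile, it asks BP_Gameplay_GM to spawn another tile.
; When the player leaves EndOfTile, the tile waits briefly, then destroys its NPCs and itself.
; Obstacle transforms use the chosen side's spawn point with random X jitter and a lift above ground.
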(event OnComponentBeginOverlap(EndOfTile)
  (params (OverlappedComponent :type Primitive%20Component%20Object%20Reference) (OtherActor :type Actor%20Object%20Reference) (OtherComp :type Primitive%20Component%20Object%20Reference) (OtherBodyIndex :type Integer) (bFromSweep :type Boolean) (SweepResult :type Hit%20Result%20Structure%20%28by%20ref%29))
  ;[1 1 1] Notify GameMode to spawn next tiles
  (Utilities|FlowControl|DoOnce false :!label _label
    (:Completed
      (if (Utilities|DoesObjectImplementInterface OtherActor "/Game/GameBP/Blueprints/Gameplay/Interfaces/I_Player.I_Player_C")
        (Default|SpawnFloorTiles (Variables|Default|GetGameMode) 1)
        (else
          (goto _label Reset))))))

(event OnComponentEndOverlap(EndOfTile)
  (params (OverlappedComponent :type Primitive%20Component%20Object%20Reference) (OtherActor :type Actor%20Object%20Reference) (OtherComp :type Primitive%20Component%20Object%20Reference) (OtherBodyIndex :type Integer))
  ;[1 0.4422 0.03086] TODO: Destroy this Tile after x seconds the player has passed it --- REVIEW case when player drives slow -- re-implement to store in GM a cache?
  (Utilities|FlowControl|DoOnce false :!label _label
    (:Completed
      (if (Utilities|DoesObjectImplementInterface OtherActor "/Game/GameBP/Blueprints/Gameplay/Interfaces/I_Player.I_Player_C")
        ;;[1 1 1] Destroy this tile and its spawned NPCs
        (Utilities|FlowControl|Delay 2.0)
        (for _array_element (Variables|Default|GetNPCsInTile)
          (Actor|DestroyActor _array_element))
        (Actor|DestroyActor)
        (else
          (goto _label Reset))))))

(event EventBeginPlay
  (bind _asbp_gameplay_gm (Utilities|Casting|CastToBP_Gameplay_GM (Game|GetGameMode)))
  (Variables|Default|SetGameMode _asbp_gameplay_gm))

(fn ConstructionScript)

(fn GetNextSpawnLocation
  (return (Math|Transform|MakeTransform (+ (Transformation|GetWorldLocation (Variables|Default|GetTileSpawnPoint)) (Math|Vector|MakeVector (LocalVariables|GetSpawnXOffset) 0.0 0.0)))))

(fn GetObstacleSpawnLoc
  (params (DirectionBias :type Integer))
  (bind _leftspawnpoint (Variables|Default|GetLeftSpawnPoint))
  (bind _rightspawnpoint (Variables|Default|GetRightSpawnPoint))
  (switch int DirectionBias ; Left or Right
    (:0
      (LocalVariables|SetRootSpawnLocation (Transformation|GetWorldLocation _leftspawnpoint))
      (LocalVariables|SetRootSpawnRotation (Transformation|GetWorldRotation _leftspawnpoint)))
    (:1
      (LocalVariables|SetRootSpawnLocation (Transformation|GetWorldLocation _rightspawnpoint))
      (LocalVariables|SetRootSpawnRotation (Transformation|GetWorldRotation _rightspawnpoint))))
  (return (Math|Transform|MakeTransform (+ (LocalVariables|GetRootSpawnLocation) (Math|Vector|MakeVector (Math|Conversions|ToFloat(Integer) (Math|Random|RandomIntegerinRange -450 450)) 0.0 5e+01)) (LocalVariables|GetRootSpawnRotation))))