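; Gameplay game mode that runs a level-based vehicle game built from chained tiles with animals.
; Difficulty, tile and animal data tables filter by level, feeding random tile spawns at each previous tile's exit until an end tile caps the count.
; It tracks time and evil-animal hits, pays rewards through the game instance, and handles vehicle purchases.
; Retry and menu reload the level, using a game instance flag to pick gameplay or menu.
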(event Custom|Event%20Play%20Level
  (bind _gameinstance (Variables|Default|GetGameInstance))
  (bind _nextlevel (Default|GetNextLevel _gameinstance))
  ;[1 1 1] Play level - increase difficulty - Call gameplay started on player controller
  (Gameplay|LoadDifficultyforLevel _nextlevel)
  (Generation|PreloadLevelData _nextlevel)
  (CallFunction|SpawnTiles 2)
  (Default|UISetCurLevel (Variables|Default|GetPlayerController) _nextlevel)
  (bind _returnvalue (Utilities|Time|SetTimerbyFunctionName 0 "TrackGameplayTime" 1.0 true))
  (Variables|Gameplay|SetGameplayTimer _returnvalue))

(event Custom|Event%20Load%20Main%20Menu
  ;[1 1 1] Load Main Menu level
  (Default|ToggleGameplayState (Variables|Default|GetGameInstance) false)
  (bind _returnvalue (Game|GetCurrentLevelName true))
  (Game|OpenLevel(byName) (Utilities|String|StringToName _returnvalue)))

(event Custom|SpawnTiles
  (params (Count :type Integer))
  ;[1 1 1] Spawn next tile and Animal
  (if (Generation|ShouldSpawnTiles)
    (for _index (range 1 Count)
      (Generation|SpawnTile))
    (bind _output_get (Variables|Generation|SetNrTilesSpawned (+ Count (Variables|Generation|GetNrTilesSpawned))))
    (Default|DEBUGUISetSpawnedTiles (Variables|Default|GetPlayerController) _output_get) ; TODO: TEMPORARY DEBUG
    ;[1 1 1] TODO: Game WIN -- Spawn final Special Tile
    (if (not (Generation|ShouldSpawnTiles))
      (Game|SpawnActorfromClass "/Game/GameBP/Blueprints/Gameplay/Tiles/BP_EndTile.BP_EndTile_C" (Variables|Generation|GetNextSpawnPoint) "Undefined" 0 (Utilities|Map|MakeMap "NewEnumerator0" "") 0))))

(event Custom|Event%20Reload%20Level
  ;[1 1 1] Play level - increase difficulty - Call gameplay started on player controller
  (Default|ToggleGameplayState (Variables|Default|GetGameInstance) true)
  (bind _returnvalue (Game|GetCurrentLevelName true))
  (Game|OpenLevel(byName) (Utilities|String|StringToName _returnvalue)))

(event Custom|Event%20Passed%20Level
  (params (PlayerHPInPercent :type Integer))
  ;[1 1 1] Play level - increase difficulty - Call gameplay started on player controller
  (bind (_moneyreward _moneylost _animalbonus) (Economy|AddMoneyRewards PlayerHPInPercent))
  (Default|EventFinishedCurrentLevel (Variables|Default|GetGameInstance))
  (Default|EventShowNextLevelUI (Variables|Default|GetPlayerController) _moneyreward _moneylost (Variables|Gameplay|GetAnimalsHit) _animalbonus))

(event Custom|Event%20Player%20Hit%20Animal
  (params (Animal :type BP%20Animal%20Object%20Reference))
  ;[1 0.7638 0] Event player has hit an evil animal -- increment counter
  (if (Variables|/Game/GameBP/Blueprints/Gameplay/Animals/BP_Animal.BP_Animal_C|GetIsEvil Animal)
    (Math|Integer|IncrementInt (Variables|Gameplay|GetAnimalsHit))))

(event Custom|Event%20Pick%20Vehicle
  (params (NewVehicle :type BP%20Vehicle%20Obj%20Object%20Reference%20%28by%20ref%29))
  ;[1 1 1] Pick Vehicle
  (Default|SetActiveVehicle (Variables|Default|GetGameInstance) NewVehicle))

(event EventBeginPlay
  ;[1 1 1] BeginPlay -> Setup references
  (bind _asbp_game_inst (Utilities|Casting|CastToBP_GameInst (Game|GetGameInstance)))
  (Variables|Default|SetGameInstance _asbp_game_inst)
  (bind _asbp_gameplay_pc (Utilities|Casting|CastToBP_Gameplay_PC (Game|GetPlayerController 0)))
  (Variables|Default|SetPlayerController _asbp_gameplay_pc)
  (if (Default|GetGameplayState (Variables|Default|GetGameInstance))
    (Default|EventPlayConsecutive (Variables|Default|GetPlayerController))
    (else
      (Default|EventShowMenu (Variables|Default|GetPlayerController)))))

(fn ConstructionScript)

(fn TrackGameplayTime
  (bind _result (Math|Integer|IncrementInt (Variables|Gameplay|GetLevelTime))
    (:%20%20
      (Default|UISetLevelTime (Variables|Default|GetPlayerController) _result))))

(fn SpawnTile
  (bind (_tiletospawn _aitospawn) (Generation|GetTiletoSpawn))
  (bind _returnvalue (Game|SpawnActorfromClass _tiletospawn (Variables|Generation|GetNextSpawnPoint) "AlwaysSpawn" 0 _aitospawn 0))
  (Variables|Generation|SetNextSpawnPoint (Default|GetNextSpawnLocation _returnvalue))
  (if (not (Variables|/Game/GameBP/Blueprints/Gameplay/Tiles/BP_MasterTile.BP_MasterTile_C|GetIsEndTile _returnvalue))
    (Default|EventInitSpawners _returnvalue)))

(fn PreloadLevelData
  (params (ForLevel :type Integer))
  (LocalVariables|SetCurrLevel ForLevel)
  (Utilities|FlowControl|Sequence
    (:then_0
      (bind _outrownames (DataTable|GetDataTableRowNames "/Game/GameData/Data/DT_TileTypes.DT_TileTypes"))
      (for _array_element _outrownames
        (bind _returnvalue (Utilities|GetDataTableRow "/Game/GameData/Data/DT_TileTypes.DT_TileTypes" _array_element)
          (:then
            (if (<= (.FromThisLevel (Utilities|Struct|BreakST_TileType _returnvalue)) (LocalVariables|GetCurrLevel))
              (Utilities|Array|Add (Variables|Generation|GetTileTypesToSpawn) _returnvalue))))))
    (:then_1
      (bind _outrownames_2 (DataTable|GetDataTableRowNames "/Game/GameData/Data/DT_AnimalTypes.DT_AnimalTypes"))
      (for _array_element_2 _outrownames_2
        (bind _returnvalue_2 (Utilities|GetDataTableRow "/Game/GameData/Data/DT_AnimalTypes.DT_AnimalTypes" _array_element_2)
          (:then
            (if (<= (.FromThisLevel (Utilities|Struct|BreakST_Animal _returnvalue_2)) (LocalVariables|GetCurrLevel))
              (Utilities|Array|Add (Variables|Generation|GetAnimalTypesToSpawn) _returnvalue_2))))))))

(fn GetTiletoSpawn
  (bind _tiletypestospawn (Variables|Generation|GetTileTypesToSpawn))
  (bind _output_get (LocalVariables|SetRandomInt (Math|Random|RandomIntegerinRange 0 (- (Utilities|Array|Length _tiletypestospawn) 1))))
  (for _array_element (.ailocations (Utilities|Array|Get(acopy) _tiletypestospawn _output_get))
    (Utilities|Map|Add (LocalVariables|GetLoc_AiToSpawn) _array_element (Generation|GetAitoSpawn)))
  (return (.tilebp (Utilities|Array|Get(acopy) _tiletypestospawn _output_get)) (LocalVariables|GetLoc_AiToSpawn)))

(fn LoadDifficultyforLevel
  (params (ForLevel :type Integer))
  (bind _outrownames (DataTable|GetDataTableRowNames "/Game/GameData/Data/DT_Difficulties.DT_Difficulties"))
  (for _array_element _outrownames
    (bind _returnvalue (Utilities|GetDataTableRow "/Game/GameData/Data/DT_Difficulties.DT_Difficulties" _array_element)
      (:then
        (if (<= ForLevel (.UpToLevel (Utilities|Struct|BreakST_Difficulty _returnvalue)))
          (Variables|Gameplay|SetLevelDifficulty _returnvalue)
          (return))))))

(fn ShouldSpawnTiles
  (return (< (Variables|Generation|GetNrTilesSpawned) (.tilecount (Variables|Gameplay|GetLevelDifficulty)))))

(fn AddMoneyRewards
  (params (PlayerHPInPercent :type Integer))
  (bind _animalshit (Variables|Gameplay|GetAnimalsHit))
  (bind _bonusperanimal (Variables|Gameplay|GetBonusPerAnimal))
  (bind _returnvalue (* _animalshit _bonusperanimal))
  (bind (_moneyearned _moneylost) (Default|UpdateMoney (Variables|Default|GetGameInstance) (/ (Math|Conversions|ToFloat(Integer) PlayerHPInPercent) 1e+02) _returnvalue))
  (return _moneyearned _moneylost _returnvalue))

(fn GetAitoSpawn
  (bind _animaltypestospawn (Variables|Generation|GetAnimalTypesToSpawn))
  (return (Utilities|Array|Get(acopy) _animaltypestospawn (Math|Random|RandomIntegerinRange 0 (- (Utilities|Array|Length _animaltypestospawn) 1)))))

(fn GetConstMaxSpeed
  (return (Variables|/Game/GameBP/Blueprints/BP_GameInst.BP_GameInst_C|GetCONST_MaxSpeed (Variables|Default|GetGameInstance))))

(fn GetConstMaxHP
  (return (Variables|/Game/GameBP/Blueprints/BP_GameInst.BP_GameInst_C|GetCONST_MaxHP (Variables|Default|GetGameInstance))))

(fn TryBuyVehicle
  (params (NewVehicle :type BP%20Vehicle%20Obj%20Object%20Reference%20%28by%20ref%29) (NewColor :type BP%20Vehicle%20Color%20Obj%20Object%20Reference%20%28by%20ref%29))
  (bind _gameinstance (Variables|Default|GetGameInstance))
  (bind _gameinstance_2 (Variables|Default|GetGameInstance))
  (bind _playerprofile (Variables|/Game/GameBP/Blueprints/BP_GameInst.BP_GameInst_C|GetPlayerProfile _gameinstance))
  (bind _money (Variables|/Game/GameBP/Blueprints/Gameplay/Objects/BP_Profile_Obj.BP_Profile_Obj_C|GetMoney _playerprofile))
  (if (Default|IsVehicleOwned (Variables|Default|GetGameInstance) (Variables|/Game/GameBP/Blueprints/Gameplay/Objects/BP_Vehicle_Obj.BP_Vehicle_Obj_C|GetId NewVehicle))
    (bind _output_get (LocalVariables|SetHasMoney (<= (Variables|/Game/GameBP/Blueprints/Gameplay/Objects/BP_VehicleColor_Obj.BP_VehicleColor_Obj_C|GetPrice NewColor) _money)))
    (if _output_get
      (Default|EventBuyColorforVehicle _gameinstance_2 NewColor NewVehicle))
    (else
      (bind _output_get_2 (LocalVariables|SetHasMoney (<= (Variables|/Game/GameBP/Blueprints/Gameplay/Objects/BP_Vehicle_Obj.BP_Vehicle_Obj_C|GetPrice NewVehicle) _money)))
      (if _output_get_2
        (Default|EventBuyVehicle _gameinstance_2 NewVehicle NewColor))))
  (return (LocalVariables|GetHasMoney)))