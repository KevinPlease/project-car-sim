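; Animal actor that travels to a destination and can be knocked over by the player, configured through an STAnimal struct.
; BeginPlay derives its spawn side from world X; on arrival it re-initializes the parent tile's spawners and destroys itself.
; A player overlap triggers mesh physics, removes the capsule and plays a hit sound once.
; Helper functions set up physical animation below the root bone, play walk sounds and disable damage.
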(event OnComponentBeginOverlap(ProxCollision)
  (params (OverlappedComponent :type Primitive%20Component%20Object%20Reference) (OtherActor :type Actor%20Object%20Reference) (OtherComp :type Primitive%20Component%20Object%20Reference) (OtherBodyIndex :type Integer) (bFromSweep :type Boolean) (SweepResult :type Hit%20Result%20Structure%20%28by%20ref%29))
  (bind _st_animal (Variables|Config|GetST_Animal))
  ;[1 1 1] Event hit by player
  (if (and (Utilities|DoesObjectImplementInterface OtherActor "/Game/GameBP/Blueprints/Gameplay/Interfaces/I_Player.I_Player_C") (not (Variables|Interaction|GetIsHit)))
    (Physics|SetSimulatePhysics (Variables|Character|GetMesh) true)
    (Components|DestroyComponent (Variables|Collision|GetCapsuleComponent))
    (Variables|Interaction|SetIsHit true)
    (Audio|SpawnSoundAttached (.hitsound _st_animal) (Variables|Character|GetMesh) (.rootbonename _st_animal) "0, 0, 0" "0, 0, 0" "KeepRelativeOffset" true 1.0 1.0 0.0 0 0)))

(event Custom|Event%20Arrived%20at%20Destination
  (bind _parenttile (Variables|Default|GetParentTile))
  ;[1 1 1] Animal arrived at desitnation
  (Utilities|IsValid _parenttile
    (:Is%20Valid
      (Default|EventInitSpawners _parenttile))
    (:Is%20Not%20Valid
      _))
  (Actor|DestroyActor))

(event EventBeginPlay
  ;[1 1 1] Begin Play
  (bind _asbp_gameplay_pc (Utilities|Casting|CastToBP_Gameplay_PC (Game|GetPlayerController 0)))
  (Variables|Default|SetPlayerController _asbp_gameplay_pc)
  (Math|Float|CompareFloat (.x (Transformation|GetWorldLocation (Variables|Character|GetMesh))) 0.0
    (:>
      (Variables|Default|SetOriginSpawnDirection "NewEnumerator1"))
    (:<
      (Variables|Default|SetOriginSpawnDirection "NewEnumerator0"))))

(fn ConstructionScript)

(fn InitPhysics
  (bind _st_animal (Variables|Config|GetST_Animal))
  (Class|PhysicalAnimationComponent|SetSkeletalMeshComponent (Variables|Default|GetPhysicalAnimation) (Variables|Character|GetMesh))
  ;[1 1 1] Config Torso Physics
  (Class|PhysicalAnimationComponent|ApplyPhysicalAnimationSettingsBelow (Variables|Default|GetPhysicalAnimation) (.rootbonename _st_animal) (Variables|Physics|GetTorsoPhysicsSettings) false)
  (Class|SkeletalMeshComponent|SetAllBodiesBelowSimulatePhysics (Variables|Character|GetMesh) (.rootbonename _st_animal) true false))

(fn DisableDamage
  (Variables|Config|SetST_Animal (Utilities|Struct|MakeST_Animal (.animalbp (Variables|Config|GetST_Animal)) 0 (.fromthislevel (Variables|Config|GetST_Animal)) (.aipathdeviation (Variables|Config|GetST_Animal)) (.walksound (Variables|Config|GetST_Animal)) (.hitsound (Variables|Config|GetST_Animal)) (.rootbonename (Variables|Config|GetST_Animal)))))

(fn MakeWalkSound
  (bind _st_animal (Variables|Config|GetST_Animal))
  (Audio|SpawnSoundAttached (.walksound _st_animal) (Variables|Character|GetMesh) (.rootbonename _st_animal) "0, 0, 0" "0, 0, 0" "KeepRelativeOffset" true 0.8 1.0 0.0 0 0))