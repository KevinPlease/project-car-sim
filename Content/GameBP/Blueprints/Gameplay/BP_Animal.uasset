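; BP_Animal is an animal character that ragdolls when a vehicle gets near it.
; On BeginPlay it records an origin spawn direction from the sign of the mesh's world X position.
; The first BP_BaseVehicle overlap with ProximityCollision enables mesh physics, destroys the capsule and sets IsHit.
; Construction copies Mass to CharacterMovement, and InitPhysics configures physical animation and simulation below the root bone.
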(event OnComponentBeginOverlap(ProximityCollision)
  (params (OverlappedComponent :type Primitive%20Component%20Object%20Reference) (OtherActor :type Actor%20Object%20Reference) (OtherComp :type Primitive%20Component%20Object%20Reference) (OtherBodyIndex :type Integer) (bFromSweep :type Boolean) (SweepResult :type Hit%20Result%20Structure%20%28by%20ref%29))
  (Utilities|Casting|CastToBP_BaseVehicle OtherActor)
  (if (not (Variables|Interaction|GetIsHit))
    (Physics|SetSimulatePhysics (Variables|Character|GetMesh) true)
    (Components|DestroyComponent (Variables|Collision|GetCapsuleComponent))
    (Variables|Interaction|SetIsHit true)))

(event EventBeginPlay
  (Math|Float|CompareFloat (.x (Transformation|GetWorldLocation (Variables|Character|GetMesh))) 0.0
    (:>
      (Variables|Default|SetOriginSpawnDirection "NewEnumerator1"))
    (:<
      (Variables|Default|SetOriginSpawnDirection "NewEnumerator0"))))

(fn ConstructionScript
  (Variables|/Script/Engine.CharacterMovementComponent|SetMass (Variables|Character|GetCharacterMovement) (Variables|Config|GetMass)))

(fn InitPhysics
  (bind _rootbonename (Variables|Physics|GetRootBoneName))
  (Class|PhysicalAnimationComponent|SetSkeletalMeshComponent (Variables|Default|GetPhysicalAnimation) (Variables|Character|GetMesh))
  ;[1 1 1] Config Torso Physics
  (Class|PhysicalAnimationComponent|ApplyPhysicalAnimationSettingsBelow (Variables|Default|GetPhysicalAnimation) _rootbonename (Variables|Physics|GetTorsoPhysicsSettings) false)
  (Class|SkeletalMeshComponent|SetAllBodiesBelowSimulatePhysics (Variables|Character|GetMesh) _rootbonename true false))