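; Base vehicle Blueprint for a player-driven vehicle that loses health when hit by animals and ends the game at zero.
; Acceleration sets throttle, forces velocity to MaxSpeed and reports noise, while stopping zeroes both throttle and velocity.
; Steering applies left or right velocity-change impulses instead of steering input.
; Hits update HP through the gameplay PlayerController, and helpers provide speed/gear strings, HP percent and body texture changes.
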(event Custom|Event%20Update%20Steering%20Direction
  (params (Direction :type ENUM_MoveDirection%20Enum :default "NewEnumerator0"))
  ;[1 1 1] Steering Input + Direction
  (Input|UpdateSteering Direction))

(event Custom|Event%20Update%20Acceleration
  (params (Amount :type Float%20%28single-precision%29))
  (bind _vehiclemovement (Variables|Default|GetVehicleMovement))
  ;[1 1 1] Throttle input
  (Class|WheeledVehicleMovementComponent|SetThrottleInput _vehiclemovement Amount)
  (Physics|SetPhysicsLinearVelocity (Variables|/Script/Engine.MovementComponent|GetUpdatedPrimitive _vehiclemovement) (Math|Vector|MakeVector (Variables|Config|GetMaxSpeed) 0.0 0.0) false "None")
  (Class|AISenseHearing|ReportNoiseEvent (Transformation|GetActorLocation) 1.0 self 0.0 "Noise"))

(event Custom|Event%20Stop
  ;[1 1 1] Auto brake when idle is seti via VehicleMovement comp settings
  (Class|WheeledVehicleMovementComponent|SetThrottleInput (Variables|Default|GetVehicleMovement) 0.0)
  (Physics|SetPhysicsLinearVelocity (Variables|/Script/Engine.MovementComponent|GetUpdatedPrimitive (Variables|Default|GetVehicleMovement)) "0, 0, 0" false "None"))

(event Collision|EventHit
  (params (MyComp :type Primitive%20Component%20Object%20Reference) (Other :type Actor%20Object%20Reference) (OtherComp :type Primitive%20Component%20Object%20Reference) (bSelfMoved :type Boolean) (HitLocation :type Vector :default "0, 0, 0") (HitNormal :type Vector :default "0, 0, 0") (NormalImpulse :type Vector :default "0, 0, 0") (Hit :type Hit%20Result%20Structure%20%28by%20ref%29))
  ;[1 1 1] Hit by enemy/animal -- handle damage received
  (bind _asbp_animal (Utilities|Casting|CastToBP_Animal Other))
  (bind _isdead (CallFunction|HandleDamageReceived (Variables|/Game/GameBP/Blueprints/Gameplay/Animals/BP_Animal.BP_Animal_C|GetHitDamage _asbp_animal)))
  (Default|DisableDamage _asbp_animal)
  (Default|UISetPlayerHP (Variables|Default|GetPlayerController) (Variables|Config|GetHealthPoints))
  ;[1 0.4422 0.03086] TEMP: until respective GameOver widget is created
  (if _isdead
    (Default|EventLost (Variables|Default|GetPlayerController))))

(event EventBeginPlay
  (bind _asbp_gameplay_pc (Utilities|Casting|CastToBP_Gameplay_PC (Game|GetPlayerController 0)))
  (Variables|Default|SetPlayerController _asbp_gameplay_pc))

(event Input|ActionEvents|InputActionHandbrake
  (params (Key :type Key%20Structure :default "None"))
  ;[0.6771 0.006217 0] Handbrake input
)

(fn ConstructionScript
  (Variables|Config|SetHealthPoints (Variables|Config|GetCoreHealthPoints)))

(fn ResetSteering
  (if (Variables|Input|GetIsSteering)
    (Class|WheeledVehicleMovementComponent|SetSteeringInput (Variables|Default|GetVehicleMovement) 0.0)))

(fn UpdateSteering
  (params (Direction :type ENUM_MoveDirection%20Enum :default "NewEnumerator0"))
  (switch Utilities|FlowControl|Switch|SwitchonENUM_MoveDirection Direction
    (:NewEnumerator0
      (LocalVariables|SetDirectionMultiplier -1.0))
    (:NewEnumerator1
      (LocalVariables|SetDirectionMultiplier 1.0)))
  (bind _output_get (LocalVariables|SetFinalImpulse (* (Variables|Input|GetSteerVelocityMultiplier) (LocalVariables|GetDirectionMultiplier))))
  (Physics|AddImpulse (Variables|/Script/Engine.MovementComponent|GetUpdatedPrimitive (Variables|Default|GetVehicleMovement)) (Math|Vector|MakeVector (/ (* (Variables|Input|GetSteerVelocityMultiplier) (LocalVariables|GetDirectionMultiplier)) 2.0) _output_get 0.0) "None" true)
  (return))

(fn UpdateHUDStrings
  ;[1 1 1] Setup String for Speed
  (Variables|HUD|SetSpeed%20Display%20String (Utilities|String|Append (Utilities|String|ToString(Integer) (Game|GetReadableSpeed)) " km/h"))
  ;[1 1 1] Setup string for Gear
  (LocalVariables|SetCurrentGear (Class|WheeledVehicleMovementComponent|GetCurrentGear (Variables|Default|GetVehicleMovement)))
  (if (Variables|Game|GetInReverseGear) ; If zero display N else display R
    (Variables|HUD|SetGear%20Display%20String "R")
    (elif (> (LocalVariables|GetCurrentGear) 0) ; If the gear is above zero use that
      (Variables|HUD|SetGear%20Display%20String (Utilities|String|ToString(Integer) (LocalVariables|GetCurrentGear)))
      (else
        (Variables|HUD|SetGear%20Display%20String "N")))))

(fn GetReadableSpeed
  (return (Math|Float|Floor (Math|Float|Absolute(Float) (* (Class|WheeledVehicleMovementComponent|GetForwardSpeed (Variables|Default|GetVehicleMovement)) 0.036)))))

(fn HandleDamageReceived
  (params (Damage :type Integer))
  (Math|Integer|CompareInt Damage (Variables|Config|GetHealthPoints)
    (:>
      (LocalVariables|SetbIsDead true :!label _label))
    (:==
      (goto _label))
    (:<
      _))
  (Variables|Config|SetHealthPoints (- (Variables|Config|GetHealthPoints) Damage))
  (return (LocalVariables|GetbIsDead)))

(fn GetHPinPercent
  (return (/ (* (Variables|Config|GetHealthPoints) 100) (Variables|Config|GetCoreHealthPoints))))

(fn UpdateMaterial
  (params (Material :type Material%20Instance%20Dynamic%20Object%20Reference))
  (Rendering|Material|SetTextureParameterValue Material "ColorMap" (Variables|Config|GetBodyTexture))
  (Rendering|Material|SetMaterialbyName (Variables|Character|GetMesh) (Variables|Config|GetBodyMaterialSlotName) Material)
  (return))

(fn GetCenterLocation
  (return (Transformation|GetWorldLocation (Variables|Default|GetCenterArrow))))