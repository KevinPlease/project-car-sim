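; Base player vehicle that drives forward, takes damage from animals and reports noise at its center every tick.
; UpdateAcceleration offsets it by MaxSpeed, reverses the camera catch-up and boosts Niagara exhaust smoke through a gate.
; Stop plays the spring-arm catch-up timeline, whose completion triggers the controller's loss event.
; Hits update the HP UI and can also trigger loss, though death is checked before damage is subtracted.
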(event Custom|Event%20Begin%20Camera%20Catchup
  (params (IsForward :type Boolean))
  ;[1 1 1] Begin camera movement behind player
  (if IsForward
    (bind _newtrack_0 (Timeline|Lerp%20Camera PlayFromStart)
      (:Update
        (Variables|/Script/Engine.SpringArmComponent|SetTargetOffset (Variables|Default|GetSpringArm) _newtrack_0))
      (:Finished
        (if IsForward
          (Default|EventLost (Variables|Default|GetPlayerController)))))
    (else
      (Timeline|Lerp%20Camera Reverse))))

(event Custom|Event%20Update%20Acceleration
  (params (DeltaTime :type Float%20%28single-precision%29))
  ;[1 1 1] Handle Movement
  (Transformation|AddActorLocalOffset (Math|Vector|MakeVector (* (Variables|Config|GetMaxSpeed) DeltaTime) 0.0 0.0) false false)
  (CallFunction|EventBeginCameraCatchup false)
  (Utilities|FlowControl|Gate false :!label _label
    (:Exit
      (CallFunction|ToggleCarSmoke true)
      (goto _label Close))))

(event Custom|Event%20Stop
  ;[1 1 1] Handle Movement
  (CallFunction|EventBeginCameraCatchup true)
  (CallFunction|ToggleCarSmoke false)
  (Utilities|FlowControl|Gate false) ; enters at Open
)

(event Collision|EventHit
  (params (MyComp :type Primitive%20Component%20Object%20Reference) (Other :type Actor%20Object%20Reference) (OtherComp :type Primitive%20Component%20Object%20Reference) (bSelfMoved :type Boolean) (HitLocation :type Vector :default "0, 0, 0") (HitNormal :type Vector :default "0, 0, 0") (NormalImpulse :type Vector :default "0, 0, 0") (Hit :type Hit%20Result%20Structure%20%28by%20ref%29))
  ;[1 1 1] Hit by enemy/animal -- handle damage received
  (bind _asbp_animal (Utilities|Casting|CastToBP_Animal Other))
  (bind _isdead (CallFunction|HandleDamageReceived (.hitdamage (Variables|/Game/GameBP/Blueprints/Gameplay/Animals/BP_Animal.BP_Animal_C|GetST_Animal _asbp_animal))))
  (Default|DisableDamage _asbp_animal)
  (Default|UISetPlayerHP (Variables|Default|GetPlayerController) (Variables|Config|GetHealthPoints))
  ;[1 0.4422 0.03086] TEMP: until respective GameOver widget is created
  (if _isdead
    (Default|EventLost (Variables|Default|GetPlayerController))))

(event EventTick
  (params (DeltaSeconds :type Float%20%28single-precision%29))
  (Class|AISenseHearing|ReportNoiseEvent (CallFunction|GetCenterLocation) 1.0 self 0.0 "None"))

(event EventBeginPlay
  (bind _asbp_gameplay_pc (Utilities|Casting|CastToBP_Gameplay_PC (Game|GetPlayerController 0)))
  (Variables|Default|SetPlayerController _asbp_gameplay_pc))

(fn ConstructionScript
  (Variables|Config|SetHealthPoints (Variables|Config|GetCoreHealthPoints)))

(fn HandleDamageReceived
  (params (Damage :type Integer))
  (Math|Integer|CompareInt 0 (Variables|Config|GetHealthPoints)
    (:>
      (LocalVariables|SetbIsDead true :!label _label))
    (:==
      (goto _label))
    (:<
      _))
  (Variables|Config|SetHealthPoints (- (Variables|Config|GetHealthPoints) Damage))
  (return (LocalVariables|GetbIsDead)))

(fn GetHpinPercent
  (return (/ (* (Variables|Config|GetHealthPoints) 100) (Variables|Config|GetCoreHealthPoints))))

(fn UpdateMaterial
  (params (Material :type Material%20Instance%20Dynamic%20Object%20Reference))
  (Rendering|Material|SetTextureParameterValue Material "ColorMap" (Variables|Config|GetBodyTexture))
  (Rendering|Material|SetMaterialbyName (Variables|Default|GetSkeletalMesh) (Variables|Config|GetBodyMaterialSlotName) Material)
  (return))

(fn GetCenterLocation
  (return (Transformation|GetWorldLocation (Variables|Default|GetCenterArrow))))

(fn ToggleCarSmoke
  (params (Enable :type Boolean))
  (bind _smokeleft (Variables|Default|GetSmokeLeft))
  (if Enable
    ;[1 1 1] TODO: Create variables for names and values
    (Niagara|SetNiagaraVariable(Float) _smokeleft "MaxSmokeSize" 75.0)
    (Niagara|SetNiagaraVariable(Float) _smokeleft "SpawnRate" 4.0)
    (else
      (Niagara|SetNiagaraVariable(Float) _smokeleft "MaxSmokeSize" 25.0)
      (Niagara|SetNiagaraVariable(Float) _smokeleft "SpawnRate" 2.0))))