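; BP_ControlledCamera is a camera Blueprint that calculates orbit-style rotation for its spring arm from yaw and pitch input.
; GetUpdatedCameraRotation clamps each input between the min and max camera speed, then adds it to the spring arm's world rotation.
; It returns the result with roll zeroed and pitch limited to a fixed range, without applying it.
; BeginPlay and the construction script are empty.
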(event EventBeginPlay)

(fn ConstructionScript)

(fn GetUpdatedCameraRotation
  (params (Yaw :type Float%20%28single-precision%29) (Pitch :type Float%20%28single-precision%29))
  (bind _springarm (Variables|Default|GetSpringArm))
  (bind _mincameraspeed (Variables|Default|GetMinCameraSpeed))
  (bind _maxcameraspeed (Variables|Default|GetMaxCameraSpeed))
  (bind _returnvalue (Transformation|GetWorldRotation _springarm))
  (bind (_roll _pitch _yaw) (Math|Rotator|BreakRotator _returnvalue))
  (return (Math|Rotator|MakeRotator 0.0 (Math|Float|Clamp(Float) (+ _pitch (Math|Float|Clamp(Float) Pitch _mincameraspeed _maxcameraspeed)) -65.0 5.0) (+ _yaw (Math|Float|Clamp(Float) Yaw _mincameraspeed _maxcameraspeed)))))