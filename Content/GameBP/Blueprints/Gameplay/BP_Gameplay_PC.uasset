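; BP_Gameplay_PC is the gameplay player controller that drives the player's vehicle and owns the HUD and pause menu.
; StartPlay caches the game mode and controlled vehicle, then creates the HUD showing HP and level time.
; Holding touch accelerates the vehicle each Tick and releasing stops it; left/right steering by touch position exists but is disconnected.
; It also pauses and resumes the game and forwards main-menu returns to the game mode.
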(event Custom|Event%20Start%20Play
  ;[1 1 1] Event BeginPlay and StartPlay for gameplay setup
  (bind _asbp_gameplay_gm (Utilities|Casting|CastToBP_Gameplay_GM (Game|GetGameMode)))
  (Variables|Default|SetGameMode _asbp_gameplay_gm)
  (bind _asbp_base_vehicle (Utilities|Casting|CastToBP_BaseVehicle (Pawn|GetControlledPawn)))
  (Variables|Default|SetPlayerCharacter _asbp_base_vehicle)
  (CallFunction|EventDrawHUD))

(event Custom|Event%20Move%20Vehicle
  (params (Direction :type Directions%20Enum :default "NewEnumerator0"))
  (bind _playercharacter (Variables|Default|GetPlayerCharacter))
  ;[1 1 1] Handles player input -- movement + stopping and steering(currently disabled)
  (switch Utilities|FlowControl|Switch|SwitchonDirections Direction
    (:NewEnumerator2
      (Default|EventUpdateAcceleration _playercharacter 1.0))
    (:NewEnumerator3
      (Default|EventStop _playercharacter))))

(event Custom|Event%20Back%20to%20MainMenu
  (Default|EventLoadMainMenu (Variables|Default|GetGameMode)))

(event EventTick
  (params (DeltaSeconds :type Float%20%28single-precision%29))
  ;[1 1 1] Handles player input -- movement + stopping and steering(currently disabled)
  (if (Variables|Input|GetIsPressed)
    (CallFunction|EventMoveVehicle "NewEnumerator2")))

(event Input|TouchEvents|InputTouch
  (params (Location :type Vector) (FingerIndex :type ETouchIndex%20Enum))
  ;[1 1 1] Handles player input -- movement + stopping and steering(currently disabled)
  (:Pressed
    (Variables|Input|SetIsPressed true))
  (:Released
    (Variables|Input|SetIsPressed false)
    (bind _output_get (Variables|Input|SetInputDirection "NewEnumerator3"))
    (CallFunction|EventMoveVehicle _output_get)))

(event Custom|Event%20Resume%20Game
  ;[1 1 1] Pause/Resume Game -- Show/hide Widget and pause/resume gameplay state
  (Game|SetGamePaused false)
  (Widget|RemovefromParent (Variables|UI|GetWB_PauseMenu)))

(event Custom|Event%20Pause%20Game
  (params (TEMP_IsGameOver :type Boolean))
  ;[1 1 1] Pause/Resume Game -- Show/hide Widget and pause/resume gameplay state
  (Game|SetGamePaused true)
  (bind _returnvalue (UserInterface|CreateWidget "/Game/GameBP/Blueprints/Gameplay/UI/HUD/WB_PauseMenu.WB_PauseMenu_C" self TEMP_IsGameOver))
  (bind _output_get (Variables|UI|SetWB_PauseMenu _returnvalue))
  (UserInterface|Viewport|AddtoViewport _output_get 1))

(event Custom|Event%20Draw%20HUD
  ;[1 1 1] Create and show HUD
  (bind _returnvalue (UserInterface|CreateWidget "/Game/GameBP/Blueprints/Gameplay/UI/HUD/WB_GameplayHUD.WB_GameplayHUD_C" self))
  (bind _output_get (Variables|UI|SetWB_GameplayHUD _returnvalue))
  (UserInterface|Viewport|AddtoViewport _output_get 0)
  (CallFunction|UISetPlayerHP (Variables|/Game/GameBP/Blueprints/Gameplay/BP_BaseVehicle.BP_BaseVehicle_C|GetHealthPoints (Variables|Default|GetPlayerCharacter))))

(fn ConstructionScript)

(fn GetTouchPositioninScreen
  (bind _centertouchradius (Variables|Input|GetCenterTouchRadius))
  (LocalVariables|SetTargetCoordinate (Math|Float|Round (.LocationX (Class|PlayerController|GetInputTouchState "Touch1"))))
  (LocalVariables|SetCenterCoordinate (/ (.SizeX (HUD|GetViewportSize)) 2))
  (if (Math|Integer|InRange(Integer) (LocalVariables|GetTargetCoordinate) (- (LocalVariables|GetCenterCoordinate) _centertouchradius) (+ (LocalVariables|GetCenterCoordinate) _centertouchradius))
    (LocalVariables|SetResultScreenPos "NewEnumerator2")
    (else
      (Math|Integer|CompareInt (LocalVariables|GetTargetCoordinate) (LocalVariables|GetCenterCoordinate) ; At this point it will aonly be bigger or smaller by over 100 pixels
        (:>
          (LocalVariables|SetResultScreenPos "NewEnumerator1"))
        (:<
          (LocalVariables|SetResultScreenPos "NewEnumerator0")))))
  (return (LocalVariables|GetResultScreenPos)))

(fn UpdateLevelTimeHUD
  (params (NewTime :type Integer))
  (Class|IHUD|UpdateTimer(Message) (Variables|UI|GetWB_GameplayHUD) NewTime))

(fn UISetPlayerHP
  (params (NewHP :type Integer))
  (Class|IHUD|UpdatePlayerHP(Message) (Variables|UI|GetWB_GameplayHUD) NewHP))