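; Tile actor that dresses itself with a left and a right tree, varying their look and placement per instance.
; Its construction script calls SetupTrees, which gives each tree a random material from TreeMaterials and a random X offset within TreeXMovementTolerance.
; The trees sit at opposite Y constraints with the same fixed rotation, and the right tree gets an extra non-negative random X nudge.
; The event graph has no active logic.
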(event EventBeginPlay
  (|CallParentFunction) ; This node is disabled and will not be called.\nDrag off pins to build functionality.
)

(event Collision|EventActorBeginOverlap
  (params (OtherActor :type Actor%20Object%20Reference)))

(event EventTick
  (params (DeltaSeconds :type Float%20%28single-precision%29)))

(fn ConstructionScript
  (|CallParentFunction)
  (CallFunction|SetupTrees))

(fn SetupTrees
  (bind _treematerials (Variables|Default|GetTreeMaterials))
  (bind _treexmovementtolerance (Variables|Default|GetTreeXMovementTolerance))
  (bind _treeyconstraint (Variables|Default|GetTreeYConstraint))
  (bind _returnvalue (Utilities|Array|Length _treematerials))
  (bind _returnvalue_2 (* _treexmovementtolerance -1))
  (bind _returnvalue_3 (- _returnvalue 1))
  (bind _returnvalue_4 (Math|Random|RandomIntegerinRange _returnvalue_2 _treexmovementtolerance))
  (bind _returnvalue_5 (Math|Random|RandomIntegerinRange 0 _returnvalue_3))
  (bind _returnvalue_6 (Math|Conversions|ToFloat(Integer) _returnvalue_4))
  (bind _output (Utilities|Array|Get(acopy) _treematerials _returnvalue_5))
  (Utilities|FlowControl|Sequence
    (:then_0
      ;[1 1 1] Color
      (Rendering|Material|SetMaterial (Variables|Default|GetTreeLeft) 0 _output)
      (Rendering|Material|SetMaterial (Variables|Default|GetTreeRight) 0 _output))
    (:then_1
      (Transformation|SetRelativeLocationAndRotation (Variables|Default|GetTreeLeft) (Math|Vector|MakeVector _returnvalue_6 _treeyconstraint 0.0) "0,70.000000, 0" false false)
      (Transformation|SetRelativeLocationAndRotation (Variables|Default|GetTreeRight) (Math|Vector|MakeVector (+ _returnvalue_6 (/ (Math|Float|Absolute(Float) _returnvalue_6) 3.0)) (* _treeyconstraint -1.0) 0.0) "0,70.000000, 0" false false))))