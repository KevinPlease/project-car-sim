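; Master grass tile actor that procedurally scatters grass on two sides, left and right, in its construction script.
; GenerateGrassFields uses nested column and row loops to add instances to the GrassLeft and GrassRight instanced mesh components, with configurable counts and spacing.
; Each new spawn transform gets a random yaw for variation.
; The right field reuses the same loop with a hardcoded negative column spacing to extend the opposite way.
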(event EventBeginPlay
  (|CallParentFunction) ; This node is disabled and will not be called.\nDrag off pins to build functionality.
)

(event Collision|EventActorBeginOverlap
  (params (OtherActor :type Actor%20Object%20Reference)))

(event EventTick
  (params (DeltaSeconds :type Float%20%28single-precision%29)))

(fn ConstructionScript
  (|CallParentFunction)
  (CallFunction|GenerateGrassFields))

(fn GenerateGrassFields
  (Utilities|FlowControl|Sequence
    (:then_0
      (LocalVariables|SetForMesh (Variables|Default|GetGrassLeft)))
    (:then_1
      (LocalVariables|SetForMesh (Variables|Default|GetGrassRight))
      (LocalVariables|SetGrassColumnDistance -5e+01)
      (LocalVariables|SetNextGrassSpawn (Math|Transform|MakeTransform "0, 0, 0" "0, 0, 0" "1,1,1"))))
  (for _index (range 0 (Variables|Default|GetGrassColumnCount))
    (for _index_2 (range 0 (Variables|Default|GetGrassRowCount))
      (Components|InstancedStaticMesh|AddInstance (LocalVariables|GetForMesh) (LocalVariables|GetNextGrassSpawn))
      (LocalVariables|SetNextGrassSpawn (Math|Transform|MakeTransform (Math|Vector|MakeVector (+ (.X (Math|Vector|BreakVector (.Location (Math|Transform|BreakTransform (LocalVariables|GetNextGrassSpawn))))) (LocalVariables|GetGrassInRow_Distance)) (* _index (LocalVariables|GetGrassColumnDistance)) 0.0) (Math|Rotator|MakeRotator 0.0 0.0 (Math|Conversions|ToFloat(Integer) (Math|Random|RandomIntegerinRange -180 180))) "1,1,1")))
    (LocalVariables|SetNextGrassSpawn (Math|Transform|MakeTransform (Math|Vector|MakeVector 0.0 (.Y (Math|Vector|BreakVector (.Location (Math|Transform|BreakTransform (LocalVariables|GetNextGrassSpawn))))) 0.0) "0, 0, 0" "1,1,1")) ; End of each row reset the x
  ))