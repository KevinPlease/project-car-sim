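; Base level tile for a track chained along X, which spawns animals from six named child-actor spawners on its left and right sides.
; InitSpawners configures spawners from the AIToSpawn map and level difficulty, then re-arms the spawn-range trigger that starts spawning on non-end tiles.
; The EndOfTile trigger notifies the player controller when passed, then on exit destroys the tile and its spawned AI after a delay.
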(event OnComponentBeginOverlap(EndOfTile)
  (params (OverlappedComponent :type Primitive%20Component%20Object%20Reference) (OtherActor :type Actor%20Object%20Reference) (OtherComp :type Primitive%20Component%20Object%20Reference) (OtherBodyIndex :type Integer) (bFromSweep :type Boolean) (SweepResult :type Hit%20Result%20Structure%20%28by%20ref%29))
  ;[1 1 1] Player passed this tile -- call PC to notify to spawn next tile OR end level
  (Utilities|FlowControl|DoOnce false :!label _label
    (:Completed
      (if (Utilities|DoesObjectImplementInterface OtherActor "/Game/GameBP/Blueprints/Gameplay/Interfaces/I_Player.I_Player_C")
        (Default|EventPassedTile (Variables|Default|GetPlayerController) (Variables|Config|GetIsEndTile))
        (else
          (goto _label Reset))))))

(event OnComponentEndOverlap(EndOfTile)
  (params (OverlappedComponent :type Primitive%20Component%20Object%20Reference) (OtherActor :type Actor%20Object%20Reference) (OtherComp :type Primitive%20Component%20Object%20Reference) (OtherBodyIndex :type Integer))
  ;[1 0.4422 0.03086] TODO: Destroy this Tile after x seconds the player has passed it --- NOT fully tested
  (Utilities|FlowControl|DoOnce false :!label _label
    (:Completed
      (if (Utilities|DoesObjectImplementInterface OtherActor "/Game/GameBP/Blueprints/Gameplay/Interfaces/I_Player.I_Player_C")
        ;;[1 1 1] Destroy this tile and its spawned NPCs
        (Utilities|FlowControl|Delay 2.0)
        (for _array_element (Variables|Default|GetAiSpawned)
          (Utilities|IsValid _array_element
            (:Is%20Valid
              (Actor|DestroyActor _array_element))))
        (Actor|DestroyActor)
        (else
          (goto _label Reset))))))

(event OnComponentBeginOverlap(AISpawnRange)
  (params (OverlappedComponent :type Primitive%20Component%20Object%20Reference) (OtherActor :type Actor%20Object%20Reference) (OtherComp :type Primitive%20Component%20Object%20Reference) (OtherBodyIndex :type Integer) (bFromSweep :type Boolean) (SweepResult :type Hit%20Result%20Structure%20%28by%20ref%29))
  ;[1 1 1] Player has approched the AI spawn range -- spawn the animals for this tile
  (Utilities|FlowControl|DoOnce true :!label _label
    (:Completed
      (if (Utilities|DoesObjectImplementInterface OtherActor "/Game/GameBP/Blueprints/Gameplay/Interfaces/I_Player.I_Player_C")
        (if (not (Variables|Config|GetIsEndTile))
          (CallFunction|EventStartSpawners))
        (else
          (goto _label Reset))))))

(event Custom|Event%20Init%20Spawners
  (bind _aitospawn (Variables|Config|GetAIToSpawn))
  (bind _keys (Utilities|Map|Keys _aitospawn))
  (for _array_element _keys
    (Default|Init (CallFunction|GetSpawnerfromName _array_element) (.Value (Utilities|Map|Find _aitospawn _array_element)) (Variables|/Game/GameBP/Blueprints/Gameplay/BP_Gameplay_GM.BP_Gameplay_GM_C|GetLevelDifficulty (Variables|/Game/GameBP/Blueprints/Gameplay/BP_Gameplay_PC.BP_Gameplay_PC_C|GetGameMode (Variables|Default|GetPlayerController))) self))
  (CallFunction|EventActivateSpawnCollision))

(event Custom|Event%20Start%20Spawners
  (bind _keys (Utilities|Map|Keys (Variables|Config|GetAIToSpawn)))
  (for _array_element _keys
    (Default|EventBeginSpawn (CallFunction|GetSpawnerfromName _array_element))))

(event Custom|Event%20Activate%20Spawn%20Collision
  ;[1 1 1] Player has approched the AI spawn range -- spawn the animals for this tile
  (Utilities|FlowControl|DoOnce true) ; enters at Reset
)

(event EventBeginPlay
  ;[1 1 1] Begin Play
  (bind _asbp_gameplay_pc (Utilities|Casting|CastToBP_Gameplay_PC (Game|GetPlayerController 0)))
  (Variables|Default|SetPlayerController _asbp_gameplay_pc))

(fn ConstructionScript
  (Variables|Config|SetSizeInWorld (* 2 (.x (Variables|/Script/Engine.SceneComponent|GetRelativeLocation (Variables|Default|GetTileSpawnPoint))))))

(fn GetNextSpawnLocation
  (bind _returnvalue (Transformation|GetActorLocation))
  (return (Math|Transform|MakeTransform (Math|Vector|MakeVector (+ (.x _returnvalue) (Variables|Config|GetSizeInWorld)) (.y _returnvalue) (.z _returnvalue)))))

(fn GetAISpawnLocation
  (params (LocationName :type ENUM_SpawnLocation%20Enum :default "NewEnumerator0"))
  (bind _leftmiddlespawner (Variables|Default|GetLeftMiddleSpawner))
  (bind _leftupspawner (Variables|Default|GetLeftUpSpawner))
  (bind _rightbottomspawner (Variables|Default|GetRightBottomSpawner))
  (bind _rightupspawner (Variables|Default|GetRightUpSpawner))
  (bind _rightmiddlespawner (Variables|Default|GetRightMiddleSpawner))
  (bind _leftbottomspawner (Variables|Default|GetLeftBottomSpawner))
  (switch Utilities|FlowControl|Switch|SwitchonENUM_SpawnLocation LocationName
    (:NewEnumerator0
      (LocalVariables|SetLocation (Transformation|GetWorldLocation _leftupspawner))
      (LocalVariables|SetRotation (Transformation|GetWorldRotation _leftupspawner)))
    (:NewEnumerator1
      (LocalVariables|SetLocation (Transformation|GetWorldLocation _leftmiddlespawner))
      (LocalVariables|SetRotation (Transformation|GetWorldRotation _leftmiddlespawner)))
    (:NewEnumerator2
      (LocalVariables|SetLocation (Transformation|GetWorldLocation _leftbottomspawner))
      (LocalVariables|SetRotation (Transformation|GetWorldRotation _leftbottomspawner)))
    (:NewEnumerator3
      (LocalVariables|SetLocation (Transformation|GetWorldLocation _rightupspawner))
      (LocalVariables|SetRotation (Transformation|GetWorldRotation _rightupspawner)))
    (:NewEnumerator4
      (LocalVariables|SetLocation (Transformation|GetWorldLocation _rightmiddlespawner))
      (LocalVariables|SetRotation (Transformation|GetWorldRotation _rightmiddlespawner)))
    (:NewEnumerator5
      (LocalVariables|SetLocation (Transformation|GetWorldLocation _rightbottomspawner))
      (LocalVariables|SetRotation (Transformation|GetWorldRotation _rightbottomspawner))))
  (return (Math|Transform|MakeTransform (LocalVariables|GetLocation) (LocalVariables|GetRotation))))

(fn GetSpawnerfromName
  (params (LocationName :type ENUM_SpawnLocation%20Enum :default "NewEnumerator0"))
  (switch Utilities|FlowControl|Switch|SwitchonENUM_SpawnLocation LocationName
    (:NewEnumerator0
      (LocalVariables|SetResult (Variables|Default|GetLeftUpSpawner)))
    (:NewEnumerator1
      (LocalVariables|SetResult (Variables|Default|GetLeftMiddleSpawner)))
    (:NewEnumerator2
      (LocalVariables|SetResult (Variables|Default|GetLeftBottomSpawner)))
    (:NewEnumerator3
      (LocalVariables|SetResult (Variables|Default|GetRightUpSpawner)))
    (:NewEnumerator4
      (LocalVariables|SetResult (Variables|Default|GetRightMiddleSpawner)))
    (:NewEnumerator5
      (LocalVariables|SetResult (Variables|Default|GetRightBottomSpawner))))
  (bind _asbp_master_spawner (Utilities|Casting|CastToBP_MasterSpawner (Variables|/Script/Engine.ChildActorComponent|GetChildActor (LocalVariables|GetResult))))
  (return _asbp_master_spawner))