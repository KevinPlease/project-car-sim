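; BP_MainMenu_PC is the main menu player controller, which shows the menu widget and relays the request to start play.
; On BeginPlay it caches BP_MainMenu_GM, stopping if the cast fails, then creates WB_MainMenu and adds it to the viewport.
; Its StartPlay event hands off to the game mode's OpenGameplayMap event.
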(event Custom|Event%20Start%20Play
  (Default|EventOpenGameplayMap (Variables|Default|GetGameMode)))

(event Custom|Event%20Show%20Main%20Menu
  (bind _returnvalue (UserInterface|CreateWidget "/Game/GameBP/Blueprints/MainMenu/UI/WB_MainMenu.WB_MainMenu_C" self))
  (bind _output_get (Variables|Default|SetWB_MainMenu _returnvalue))
  (UserInterface|Viewport|AddtoViewport _output_get 0))

(event EventBeginPlay
  (bind _asbp_main_menu_gm (Utilities|Casting|CastToBP_MainMenu_GM (Game|GetGameMode)))
  (Variables|Default|SetGameMode _asbp_main_menu_gm)
  (CallFunction|EventShowMainMenu))

(fn ConstructionScript)