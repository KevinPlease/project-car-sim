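; BP_Utils is a utility Blueprint with helpers for unique random integers and vehicle ownership filtering.
; RandomUniqueIntInRange recursively retries when a roll is in the passed list, otherwise appends CurInt, with no guard for an exhausted range.
; Its Contains check re-rolls the random node rather than testing CurInt, so uniqueness is not guaranteed.
; FilterOwnVehicles builds a map, keyed by Id, of the vehicles flagged IsOwned.
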(fn RandomUniqueIntinRange
  (params (Min :type Integer) (Max :type Integer) (CurIntsPassed :type Array%20of%20Integers))
  (bind _returnvalue (Math|Random|RandomIntegerinRange Min Max))
  (LocalVariables|SetCurInt _returnvalue)
  (if (Utilities|Array|ContainsItem CurIntsPassed _returnvalue)
    (LocalVariables|SetCurInt (CallFunction|RandomUniqueIntinRange Min Max CurIntsPassed))
    (else
      (Utilities|Array|Add CurIntsPassed (LocalVariables|GetCurInt))))
  (return (LocalVariables|GetCurInt)))

(fn FilterOwnVehicles
  (params (AllVehicles :type Map%20of%20Integers%20to%20Objects))
  (bind _values (Utilities|Map|Values AllVehicles))
  (for _array_element _values
    (if (Variables|/Game/GameBP/Blueprints/Gameplay/Objects/BP_Vehicle_Obj.BP_Vehicle_Obj_C|GetIsOwned _array_element)
      (Utilities|Map|Add (LocalVariables|GetLocOwnVehicles) (Variables|/Game/GameBP/Blueprints/Gameplay/Objects/BP_Vehicle_Obj.BP_Vehicle_Obj_C|GetId _array_element) _array_element)))
  (return (LocalVariables|GetLocOwnVehicles)))